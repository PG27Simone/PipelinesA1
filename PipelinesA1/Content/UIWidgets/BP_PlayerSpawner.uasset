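; BP_PlayerSpawner moves the player character to a selected checkpoint when play begins.
; On BeginPlay it scans every BP_Checkpoints actor and compares its display name to SelectedSpawnPointName.
; A match sets the player's location and rotation to that checkpoint's transform, without sweep or teleport physics.
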(event EventBeginPlay
  (bind _returnvalue (Game|GetPlayerCharacter 0))
  (bind _outactors (Actor|GetAllActorsOfClass "/Game/UIWidgets/BP_Checkpoints.BP_Checkpoints_C"))
  (for _array_element _outactors
    (if (Utilities|Enum|Equal(Enum) (Utilities|GetDisplayName _array_element) (Variables|Default|GetSelectedSpawnPointName))
      (Transformation|SetActorLocation _returnvalue (Transformation|GetActorLocation _array_element) false false)
      (Transformation|SetActorRotation _returnvalue (Transformation|GetActorRotation _array_element)))))

(fn ConstructionScript)